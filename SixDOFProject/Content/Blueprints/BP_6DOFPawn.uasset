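; Player pawn with six-degree-of-freedom flight and a walk mode, driven by axis inputs for movement, pitch, yaw and roll plus a speed boost.
; Jump switches from Fly to Walk when the surface is walkable; in Walk it jumps on the ground or returns to Fly in the air.
; While flying, a camera trace recolors the crosshair widget on hits and walkability toggles its visibility, using paired DoOnce gates to update only on changes.
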(event `self.ReceiveTick`
  (params (DeltaSeconds :type "Float (single-precision)"))
  (bind _returnvalue (`GameplayStatics.GetPlayerCameraManager` 0))
  (bind _returnvalue_2 (`PlayerCameraManager.GetCameraLocation` _returnvalue))
  (if (`|EnumEquality` (`SixDOFMovementComponent.CustomMovementMode` (`self.MovementComponent`)) "ECMM_Fly")
    (`|ExecutionSequence`
      (:`then_0`
        (bind (_outhit _returnvalue_3) (`KismetSystemLibrary.LineTraceSingle` _returnvalue_2 (+ _returnvalue_2 (* (`KismetMathLibrary.GetForwardVector` (`PlayerCameraManager.GetCameraRotation` _returnvalue)) (`self.Trace length`))) "TraceTypeQuery1"))
        (if _returnvalue_3
          (`/Engine/EditorBlueprintResources/StandardMacros.DoOnce` false :!label _label
            (:`Completed`
              (`/Game/Blueprints/WG_Crosshair.Set Crosshair Image Color` (`self.CrosshairWG_Ref`) (struct :`R` 1.0 :`G` 0.045801 :`A` 0.75))
              (goto _label_2 :!via `Reset`)))
          (else
            (`/Engine/EditorBlueprintResources/StandardMacros.DoOnce` false :!label _label_2
              (:`Completed`
                (`/Game/Blueprints/WG_Crosshair.Set Crosshair Image Color` (`self.CrosshairWG_Ref`) (struct :`G` 0.803114 :`B` 1.0 :`A` 0.75))
                (goto _label :!via `Reset`))))))
      (:`then_1`
        (if (`SixDOFMovementComponent.CanWalkOnSurface` (`self.MovementComponent`))
          (`/Engine/EditorBlueprintResources/StandardMacros.DoOnce` false :!label _label_3
            (:`Completed`
              (`/Game/Blueprints/WG_Crosshair.Set Crosshair Image Visible` (`self.CrosshairWG_Ref`) true)
              (goto _label_4 :!via `Reset`)))
          (else
            _)))))
  (`/Engine/EditorBlueprintResources/StandardMacros.DoOnce` false :!label _label_4
    (:`Completed`
      (`/Game/Blueprints/WG_Crosshair.Set Crosshair Image Visible` (`self.CrosshairWG_Ref`) false)
      (goto _label_3 :!via `Reset`))))

(event `self.ReceiveBeginPlay`
  (bind _returnvalue (`|CreateWidget` "/Game/Blueprints/WG_Crosshair.WG_Crosshair_C" (`GameplayStatics.GetPlayerController` 0)))
  (bind _output_get (set `self.CrosshairWG_Ref` _returnvalue))
  (`UserWidget.AddToViewport` _output_get 0))

(event `InputAxis|MoveForward`
  (params (AxisValue :type "Float (single-precision)"))
  (`self.AddForwardMovementInput` AxisValue))

(event `InputAxis|MoveRight`
  (params (AxisValue :type "Float (single-precision)"))
  (`self.AddRightMovementInput` AxisValue))

(event `InputAxis|MoveUp`
  (params (AxisValue :type "Float (single-precision)"))
  (`self.AddUpMovementInput` AxisValue))

(event `InputAxis|PitchUp`
  (params (AxisValue :type "Float (single-precision)"))
  (`self.AddPawnPitchInput` (`self.Rotation Rate`) (* AxisValue -1.0)))

(event `InputAxis|YawRight`
  (params (AxisValue :type "Float (single-precision)"))
  (`self.AddPawnYawInput` (`self.Rotation Rate`) AxisValue))

(event `InputAxis|RollRight`
  (params (AxisValue :type "Float (single-precision)"))
  (`self.AddPawnRollInput` (`self.Rotation Rate`) AxisValue))

(event `InputAction|Jump`
  (params (Key :type "Key Structure" :default "AnyKey"))
  (:`Pressed`
    (switch `ECustomMovementMode` (`SixDOFMovementComponent.CustomMovementMode` (`self.MovementComponent`))
      (:`ECMM_Fly`
        (if (`SixDOFMovementComponent.CanWalkOnSurface` (`self.MovementComponent`))
          (`SixDOFMovementComponent.SetCustomMovementMode` (`self.MovementComponent`) "ECMM_Walk" false)))
      (:`ECMM_Walk`
        (if (`NavMovementComponent.IsMovingOnGround` (`self.MovementComponent`))
          (`self.Jump`)
          (else
            (`SixDOFMovementComponent.SetCustomMovementMode` (`self.MovementComponent`) "ECMM_Fly" true)))))))

(event `InputAction|Boost`
  (params (Key :type "Key Structure" :default "AnyKey"))
  (:`Pressed`
    (`self.SpeedBoost`))
  (:`Released`
    (`self.StopSpeedBoost`)))

(fn `UserConstructionScript`)