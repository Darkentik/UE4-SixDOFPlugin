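; Six-degree-of-freedom player pawn that switches between free flight and walking on surfaces.
; Axis inputs drive translation and frame-rate-scaled pitch, yaw and roll, while Boost applies a speed boost when held.
; Jump switches flight to walking on a walkable surface, jumps when grounded, or returns to flight when airborne in Walk mode.
; A crosshair widget shows a button prompt whenever landing is possible.
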(event `self.ReceiveBeginPlay`
  (bind _returnvalue (`|CreateWidget` "/Game/Widget/Cross.Cross_C" (`GameplayStatics.GetPlayerController` 0)))
  (bind _output_get (set `self.CrosshairWG_Ref` _returnvalue))
  (`UserWidget.AddToViewport` _output_get 0))

(event `self.ReceiveTick`
  (params (DeltaSeconds :type "Float (single-precision)"))
  (if (and (`SixDOFMovementComponent.CanWalkOnSurface` (`self.MovementComponent`)) (`|EnumEquality` (`SixDOFMovementComponent.CustomMovementMode` (`self.MovementComponent`)) "ECMM_Fly"))
    (`Widget.SetVisibility` (`/Game/Widget/Cross.PressA` (`self.CrosshairWG_Ref`)) "Visible")
    (else
      (`Widget.SetVisibility` (`/Game/Widget/Cross.PressA` (`self.CrosshairWG_Ref`)) "Hidden"))))

(event `InputAxis|MoveForward`
  (params (AxisValue :type "Float (single-precision)"))
  (`self.AddForwardMovementInput` AxisValue))

(event `InputAxis|MoveRight`
  (params (AxisValue :type "Float (single-precision)"))
  (`self.AddRightMovementInput` AxisValue))

(event `InputAxis|MoveUp`
  (params (AxisValue :type "Float (single-precision)"))
  (`self.AddUpMovementInput` AxisValue))

(event `InputAxis|PitchUp`
  (params (AxisValue :type "Float (single-precision)"))
  (`self.AddPawnPitchInput` (* (`self.PitchRotationSpeed`) (`GameplayStatics.GetWorldDeltaSeconds`) -1.0) AxisValue))

(event `InputAxis|YawRight`
  (params (AxisValue :type "Float (single-precision)"))
  (`self.AddPawnYawInput` (* (`self.YawRotationSpeed`) (`GameplayStatics.GetWorldDeltaSeconds`)) AxisValue))

(event `InputAxis|RollRight`
  (params (AxisValue :type "Float (single-precision)"))
  (`self.AddPawnRollInput` (* (`self.RollRotationSpeed`) (`GameplayStatics.GetWorldDeltaSeconds`)) AxisValue))

(event `InputAction|Jump`
  (params (Key :type "Key Structure" :default "AnyKey"))
  (:`Pressed`
    (switch `ECustomMovementMode` (`SixDOFMovementComponent.CustomMovementMode` (`self.MovementComponent`))
      (:`ECMM_Fly`
        (if (`SixDOFMovementComponent.CanWalkOnSurface` (`self.MovementComponent`))
          (`SixDOFMovementComponent.SetCustomMovementMode` (`self.MovementComponent`) "ECMM_Walk" false)))
      (:`ECMM_Walk`
        (if (`NavMovementComponent.IsMovingOnGround` (`self.MovementComponent`))
          (`self.Jump`)
          (else
            (`SixDOFMovementComponent.SetCustomMovementMode` (`self.MovementComponent`) "ECMM_Fly" true)))))))

(event `InputAction|Boost`
  (params (Key :type "Key Structure" :default "AnyKey"))
  (:`Pressed`
    (`self.SpeedBoost`))
  (:`Released`
    (`self.StopSpeedBoost`)))

(fn `UserConstructionScript`)